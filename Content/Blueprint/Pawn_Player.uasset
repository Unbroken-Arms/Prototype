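; Player pawn for a two-sided multiplayer game that moves along a spline path and interacts with or grabs objects under the cursor.
; A timeline, rate-scaled by path length for constant speed, drives forward and backward movement.
; Interactions go through server and multicast events to BPI_Interaction targets, while misses trigger a zoom timeline that alters the other player's FOV.
; A scene capture renders each side's view to its own render target.
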(event `self.ReceiveControllerChanged`
  (params (OldController :type "Controller Object Reference") (NewController :type "Controller Object Reference"))
  ;[1 0.8922 0.3718] Add Input Context
  (`self.AddMappingContextAndHUD` NewController))

(event `EnhancedInput|/Game/Blueprint/Input/InA_Forward`
  (params (ActionValue :type Boolean) (ElapsedSeconds :type "Float (double-precision)") (TriggeredSeconds :type "Float (double-precision)") (InputAction :type "InputAction Object Reference" :default "/Game/Blueprint/Input/InA_Forward.InA_Forward"))
  ;[1 0.3614 0.2516] Movement
  (:`Started`
    (bind (_direction _alpha) (`Timeline|Slider` :!label _label)
      (:`Update`
        (`self.Move` _alpha))))
  (:`Completed`
    (goto _label :!via `Stop`)))

(event `EnhancedInput|/Game/Blueprint/Input/InA_Backward`
  (params (ActionValue :type Boolean) (ElapsedSeconds :type "Float (double-precision)") (TriggeredSeconds :type "Float (double-precision)") (InputAction :type "InputAction Object Reference" :default "/Game/Blueprint/Input/InA_Backward.InA_Backward"))
  ;[1 0.3614 0.2516] Movement
  (:`Started`
    (goto _label :!via `Reverse`))
  (:`Completed`
    (goto _label :!via `Stop`)))

(event `S_Interact`
  (params (Target :type "/Game/Blueprint/BPI_Interaction Interface") (Caller :type "Array of Object Object Reference (by ref)"))
  ;[0.2091 0.3434 1] Interaction Server and Multicast
  (`self.M_Interact` Target Caller))

(event `S_Grab`
  (params (Target :type "/Game/Blueprint/BPI_Interaction Interface") (Caller :type "Array of Object Object Reference (by ref)") (Interact :type Boolean))
  ;[0.2091 0.3434 1] Interaction Server and Multicast
  (`self.M_Grab` Target Caller Interact))

(event `EnhancedInput|/Game/Blueprint/Input/InA_Interact`
  (params (ActionValue :type Boolean) (ElapsedSeconds :type "Float (double-precision)") (TriggeredSeconds :type "Float (double-precision)") (InputAction :type "InputAction Object Reference" :default "/Game/Blueprint/Input/InA_Interact.InA_Interact"))
  ;[1 0.3445 0.1129] Interaction
  (:`Triggered`
    (`self.Interact` "NewEnumerator0" ActionValue)))

(event `EnhancedInput|/Game/Blueprint/Input/InA_Grab`
  (params (ActionValue :type Boolean) (ElapsedSeconds :type "Float (double-precision)") (TriggeredSeconds :type "Float (double-precision)") (InputAction :type "InputAction Object Reference" :default "/Game/Blueprint/Input/InA_Grab.InA_Grab"))
  ;[1 0.3445 0.1129] Interaction
  (:`Started`
    (`self.Interact` "NewEnumerator1" ActionValue :!label _label_2))
  (:`Completed`
    (goto _label_2)))

(event `M_Interact`
  (params (Target :type "/Game/Blueprint/BPI_Interaction Interface") (Caller :type "Array of Object Object Reference (by ref)"))
  ;[0.2091 0.3434 1] Interaction Server and Multicast
  (`/Game/Blueprint/BPI_Interaction.Interact` Target Caller))

(event `M_Grab`
  (params (Target :type "/Game/Blueprint/BPI_Interaction Interface") (Caller :type "Array of Object Object Reference (by ref)") (Interact :type Boolean))
  ;[0.2091 0.3434 1] Interaction Server and Multicast
  (`/Game/Blueprint/BPI_Interaction.Grab` Target Caller Interact))

(event `S_ChangeFOV`
  (params (`Field of View` :type "Float (single-precision)"))
  ;[1 0.1622 0.8822] Bad Interaction Server and Multicast
  (`self.M_ChangeFOV` `Field of View`))

(event `BadInteraction`
  (bind _data (`self.Data`))
  ;[1 0.01752 0] Bad Interaction
  (if (`self.InAnimation`)
    (bind (_direction _alpha) (`Timeline|Zoom` :`NewTime` 0.15 :!via `SetNewTime` :!label _label_3)
      (:`Update`
        (`self.S_ChangeFOV` (`KismetMathLibrary.Lerp` (`/Game/Blueprint/Data/PDA_Player.MinFOV` _data) (`/Game/Blueprint/Data/PDA_Player.BaseFOV` _data) _alpha)))
      (:`Finished`
        (set `self.InAnimation` false)))
    (else
      (set `self.InAnimation` true)
      (goto _label_3 :!via `PlayFromStart`))))

(event `M_ChangeFOV`
  (params (`Field of View` :type "Float (single-precision)"))
  ;[1 0.1622 0.8822] Bad Interaction Server and Multicast
  (`self.ChangeFOV` (`self.OtherPlayer`) `Field of View`))

(fn `AddMappingContextAndHUD`
  (params (Controller :type "Controller Object Reference"))
  (`/Engine/EditorBlueprintResources/StandardMacros.IsValid` Controller
    (:`Is Valid`
      (if (`Controller.IsLocalController` Controller)
        (bind _aspc_player (cast `/Game/Blueprint/PC_Player` Controller))
        (`EnhancedInputSubsystemInterface.AddMappingContext` (pcsubsystem `EnhancedInputLocalPlayerSubsystem` _aspc_player) "/Game/Blueprint/Input/InMC_Movement.InMC_Movement" 0 (struct))
        (`/Game/Blueprint/PC_Player.AddHUD` _aspc_player (`self.PlayerSide`))))))

(fn `ChangeFOV`
  (params (`Field of View` :type "Float (single-precision)"))
  (bind _output_get (set `SceneCaptureComponent2D.FOVAngle` `Field of View` (`self.SceneCaptureComponent2D`)))
  (`CameraComponent.SetFieldOfView` (`self.Camera`) _output_get))

(fn `GetInitialTransform`
  (params (Path :type "/Game/Blueprint/BP_Path Object Reference"))
  (returns (Transform :type "Transform Structure"))
  (bind _spline (`/Game/Blueprint/BP_Path.Spline` Path))
  (return (`SplineComponent.GetTransformAtDistanceAlongSpline` _spline (`KismetMathLibrary.SelectFloat` (`SplineComponent.GetSplineLength` _spline) 0.0 (`/Game/Blueprint/BP_Path.FromEnd` Path)) "World" false)))

(fn `GetResultUnderCenterOfScreen`
  (returns (HitActor :type "Actor Object Reference"))
  (bind _camera (`self.Camera`))
  (bind _returnvalue (`SceneComponent.K2_GetComponentLocation` _camera))
  (bind _outhit (`KismetSystemLibrary.LineTraceSingle` _returnvalue (+ _returnvalue (* (`SceneComponent.GetForwardVector` _camera) 1000000)) "TraceTypeQuery1"))
  (return (`.HitActor` (`GameplayStatics.BreakHitResult` _outhit))))

(fn `GetResultUnderCursor`
  (returns (HitActor :type "Actor Object Reference"))
  (return (`.HitActor` (`GameplayStatics.BreakHitResult` (`PlayerController.GetHitResultUnderCursorByChannel` (`GameplayStatics.GetPlayerController` 0) "TraceTypeQuery1" true)))))

(fn `GetTimeLinePlayRate`
  (returns (ReturnValue :type "Float (double-precision)"))
  (return (/ 1.0 (/ (`SplineComponent.GetSplineLength` (`/Game/Blueprint/BP_Path.Spline` (`self.Path`))) (`/Game/Blueprint/Data/PDA_Player.MoveSpeed` (`self.Data`))))))

(fn `Interact`
  (params (Action :type "/Game/Blueprint/Enum/Enum_Action Enum" :default "NewEnumerator0") (Start :type Boolean))
  (bind _array (`|MakeArray` self :!type "Object Object Reference"))
  (bind _asbpi_interaction (cast `/Game/Blueprint/BPI_Interaction` (`self.GetResultUnderCursor`))
    (:`then`
      (switch `/Game/Blueprint/Enum/Enum_Action` Action
        (:`NewEnumerator0`
          (if Start
            (`self.S_Interact` _asbpi_interaction _array)))
        (:`NewEnumerator1`
          (`self.S_Grab` _asbpi_interaction _array Start))))
    (:`CastFailed`
      (`self.BadInteraction`))))

(fn `Move`
  (params (Alpha :type "Float (double-precision)"))
  (bind _path (`self.Path`))
  (bind _spline (`/Game/Blueprint/BP_Path.Spline` _path))
  (bind _returnvalue (`SplineComponent.GetSplineLength` _spline))
  (`self.K2_SetActorTransform` (`SplineComponent.GetTransformAtDistanceAlongSpline` _spline (`KismetMathLibrary.SelectFloat` (`KismetMathLibrary.Lerp` _returnvalue 0.0 Alpha) (`KismetMathLibrary.Lerp` 0.0 _returnvalue Alpha) (`/Game/Blueprint/BP_Path.FromEnd` _path)) "World" false)))

(fn `UserConstructionScript`
  (bind _path (`self.Path`))
  (bind _basefov (`/Game/Blueprint/Data/PDA_Player.BaseFOV` (`self.Data`)))
  (`/Engine/EditorBlueprintResources/StandardMacros.IsValid` _path
    (:`Is Valid`
      (`self.K2_SetActorTransform` (`self.GetInitialTransform` _path))
      (`TimelineComponent.SetPlayRate` (`self.Slider`) (`self.GetTimeLinePlayRate`))
      (set `SceneCaptureComponent2D.TextureTarget` (select `/Game/Blueprint/Enum/Enum_Player` (`self.PlayerSide`) :`NewEnumerator0` "/Game/Material/Render/RT_ScreenA.RT_ScreenA" :`NewEnumerator1` "/Game/Material/Render/RT_ScreenB.RT_ScreenB" :!type "TextureRenderTarget2D Object Reference") (`self.SceneCaptureComponent2D`))
      (`CameraComponent.SetFieldOfView` (`self.Camera`) _basefov)
      (set `SceneCaptureComponent2D.FOVAngle` _basefov (`self.SceneCaptureComponent2D`)))))