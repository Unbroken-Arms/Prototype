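; BP_Item is a data-driven item that can be interacted with and grabbed, with its look and behavior both set by its Data.
; The construction script applies the mesh, materials, scale and offset, then constructs a Reaction object from the class in Data.
; Ready gives the Reaction the GameMode and begins it, while Interact, Grab and Destroyed delegate to it.
; Interact and Grab also add the item uniquely to the caller.
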(event `self.ReceiveDestroyed`
  (`/Game/Blueprint/Data/Reaction/O_Reaction.Destroy` (`self.Reaction`)))

(event `Ready`
  (bind _reaction (`self.Reaction`))
  (set `/Game/Blueprint/Data/Reaction/O_Reaction.GameMode` (`GameplayStatics.GetGameMode`) _reaction)
  (`/Game/Blueprint/Data/Reaction/O_Reaction.BeginPlay` _reaction))

(event `/Game/Blueprint/BPI_Interaction.Interact`
  (params (Caller :type "Array of Object Object Reference (by ref)"))
  (`KismetArrayLibrary.Array_AddUnique` Caller self)
  (`/Game/Blueprint/BPI_Interaction.Interact` (`self.Reaction`) Caller))

(event `/Game/Blueprint/BPI_Interaction.Grab`
  (params (Caller :type "Array of Object Object Reference (by ref)") (Interact :type Boolean))
  (`KismetArrayLibrary.Array_AddUnique` Caller self)
  (`/Game/Blueprint/BPI_Interaction.Grab` (`self.Reaction`) Caller Interact))

(event `CreateReaction`
  (bind _returnvalue (`|GenericCreateObject` (`/Game/Blueprint/Data/PDA_Item.Reaction` (`self.Data`))))
  (bind _output_get (set `self.Reaction` _returnvalue))
  (`/Game/Blueprint/Data/Reaction/O_Reaction.OverrideItem` _output_get))

(fn `UserConstructionScript`
  (bind _data (`self.Data`))
  (bind _mesh (`self.Mesh`))
  (`StaticMeshComponent.SetStaticMesh` _mesh (`/Game/Blueprint/Data/PDA_Item.Mesh` _data))
  (for (_array_element _array_index) (`/Game/Blueprint/Data/PDA_Item.Material` _data)
    (`PrimitiveComponent.SetMaterial` _mesh _array_index _array_element))
  (`SceneComponent.SetWorldScale3D` _mesh (`/Game/Blueprint/Data/PDA_Item.Scale` _data))
  (`SceneComponent.K2_AddWorldOffset` _mesh (`/Game/Blueprint/Data/PDA_Item.Offset` _data) false false)
  (`self.CreateReaction`))