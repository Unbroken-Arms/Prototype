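; Game mode that assigns each joining player to a pre-placed Pawn_Player by join order and starts the level's items.
; On a new player, the controller is added to a Players list and possesses the pawn at the same index.
; When the second player joins, every BP_Item is told it is ready.
; A helper function rebuilds and returns the player controller list from the current player count.
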(event `self.HandleStartingNewPlayer`
  (params (NewPlayer :type "PlayerController Object Reference"))
  (bind _returnvalue (`KismetArrayLibrary.Array_AddUnique` (`self.Players`) NewPlayer))
  (bind _outactors (`GameplayStatics.GetAllActorsOfClass` "/Game/Blueprint/Pawn_Player.Pawn_Player_C"))
  (`Controller.Possess` NewPlayer (`|GetArrayItem` _outactors _returnvalue))
  (if (== _returnvalue 1)
    (bind _outactors_2 (`GameplayStatics.GetAllActorsOfClass` "/Game/Blueprint/BP_Item.BP_Item_C"))
    (for _array_element _outactors_2
      (`/Game/Blueprint/BP_Item.Ready` _array_element))))

(fn `GetPlayerController`
  (returns (PlayerControllers :type "Array of PlayerController Object Reference"))
  (locals (Players :type "Array of PlayerController Object Reference"))
  (bind _returnvalue (`self.GetNumPlayers`))
  (for _index (range 1 (+ _returnvalue 1))
    (`KismetArrayLibrary.Array_AddUnique` (`local.Players`) (`GameplayStatics.GetPlayerController` (- _index 1))))
  (return (`local.Players`)))

(fn `UserConstructionScript`)