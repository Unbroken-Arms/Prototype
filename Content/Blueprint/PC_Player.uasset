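; Player controller that sets up the HUD and records the player's side when it possesses a pawn.
; On every possess it calls AddHUD, which creates a UI_HUD widget, adds it to the viewport and stores it, only for a local controller.
; It then casts the pawn to Pawn_Player and copies its PlayerSide onto the controller.
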(event `self.ReceivePossess`
  (params (PossessedPawn :type "Pawn Object Reference"))
  ;[0.2266 0.6709 1] Add HUD
  (`self.AddHUD`)
  (bind _aspawn_player (cast `/Game/Blueprint/Pawn_Player` PossessedPawn))
  (set `self.Player Side` (`/Game/Blueprint/Pawn_Player.PlayerSide` _aspawn_player)))

(event `AddHUD`
  ;[0.2266 0.6709 1] Add HUD
  (if (`self.IsLocalPlayerController`)
    (bind _returnvalue (`|CreateWidget` "/Game/Blueprint/UI/UI_HUD.UI_HUD_C" self))
    (`UserWidget.AddToViewport` _returnvalue 0)
    (set `self.HUD` _returnvalue)))

(fn `UserConstructionScript`)